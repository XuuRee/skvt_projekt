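; BP_EMP_Sphere is a one-shot EMP trigger that destroys nearby electric actors.
; The first overlap with its Box reveals the hidden Sphere mesh, scales it up and derives a blast radius from that scale.
; A sphere overlap query on WorldDynamic objects then destroys every actor implementing BPI_Electric.
; Debug sphere drawing and print strings show the blast area and each result.
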(event `self.ReceiveBeginPlay`)

(event `self.Box.OnComponentBeginOverlap`
  (params (OverlappedComponent :type "PrimitiveComponent Object Reference") (OtherActor :type "Actor Object Reference") (OtherComp :type "PrimitiveComponent Object Reference") (OtherBodyIndex :type Integer) (bFromSweep :type Boolean) (SweepResult :type "HitResult Structure (by ref)"))
  (if (not (`self.EMPUsed`))
    (`SceneComponent.SetVisibility` (`self.Sphere`) true false)
    (set `self.EMPUsed` true)
    (bind _output_get (set `self.SphereScale` (`KismetMathLibrary.MakeVector` 10.0 10.0 10.0)))
    (`SceneComponent.SetWorldScale3D` (`self.Sphere`) _output_get)
    (bind _float (`self.Get Sphere Radius` _output_get))
    (`KismetSystemLibrary.DrawDebugSphere` (`SceneComponent.K2_GetComponentLocation` (`self.Sphere`)) _float 12 (struct :`R` 1.0 :`G` 1.0 :`B` 1.0 :`A` 1.0) 50.0)
    (bind _outactors (`KismetSystemLibrary.SphereOverlapActors` (`SceneComponent.K2_GetComponentLocation` (`self.Sphere`)) _float (`|MakeArray` "ObjectTypeQuery2" :!type "EObjectTypeQuery Enum")))
    (bind _output_get_2 (set `self.AllActors` _outactors))
    (for _array_element _output_get_2
      (bind _asbpi_electric (cast `/Game/Skvt/Blueprints/BPI_Electric` _array_element)
        (:`then`
          (`KismetSystemLibrary.PrintString` "Hello")
          (`/Game/Skvt/Blueprints/BPI_Electric.Destroy` _asbpi_electric))
        (:`CastFailed`
          (`KismetSystemLibrary.PrintString` "Failed"))))))

(fn `Get Sphere Radius`
  (params (Scale :type "Vector Structure"))
  (returns (Float :type "Float (double-precision)"))
  (return (/ (* (.x Scale) 100.0) 2.0)))

(fn `MultiplyVector`
  (params (Vector :type "Vector Structure") (Float :type "Float (double-precision)"))
  (returns (Result :type "Vector Structure"))
  (return (`KismetMathLibrary.MakeVector` (* (.x Vector) Float) (* (.y Vector) Float) (* (.z Vector) Float))))

(fn `UserConstructionScript`
  (`SceneComponent.SetVisibility` (`self.Sphere`) false false))